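; Camera pawn with a spring arm that can pan, zoom and follow a selected actor.
; ChangeSelectChar stores the target and starts a looping timer that snaps the spring arm to its location.
; Zoom adjusts clamped arm length, while panning offsets the pawn in world X/Y, both scaled by frame time.
; Panning clears a timer named CameraMoveToSelectChar, which differs from the follow timer's CameraMoveToTarget.
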(fn ConstructionScript)

(fn ChangeSelectChar
  (params (TargetActor :type Actor%20Object%20Reference))
  (Variables|Default|SetTargetActor TargetActor)
  (Utilities|Time|SetTimerbyFunctionName 0 "CameraMoveToTarget" 0.01 true))

(fn CameraMovetoTarget
  (bind _targetactor (Variables|Default|GetTargetActor)
    (:then
      (Transformation|SetWorldLocation (Variables|Default|GetSpringArm) (Transformation|GetActorLocation _targetactor) false false))
    (:else)))

(fn CameraZoom
  (params (ActionValue :type Float%20%28double-precision%29))
  (bind _springarm (Variables|Default|GetSpringArm))
  (Variables|/Script/Engine.SpringArmComponent|SetTargetArmLength _springarm (Math|Float|Clamp(Float) (- (Variables|/Script/Engine.SpringArmComponent|GetTargetArmLength _springarm) (* ActionValue (Variables|Default|GetZoomSpeed) (Utilities|Time|GetWorldDeltaSeconds))) (Variables|Default|GetMinZoom) (Variables|Default|GetMaxZoom))))

(fn CameraMove
  (params (X :type Float%20%28double-precision%29) (Y :type Float%20%28double-precision%29))
  (bind _returnvalue (Utilities|Time|GetWorldDeltaSeconds))
  (bind _movespeed (Variables|Default|GetMoveSpeed))
  (Utilities|Time|ClearTimerbyFunctionName 0 "CameraMoveToSelectChar")
  (Transformation|AddActorWorldOffset (Math|Vector|MakeVector (* X _movespeed _returnvalue) (* Y _movespeed _returnvalue) 0.0)))