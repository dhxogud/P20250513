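; BP_BaseUnit is a base unit Blueprint for a turn-based game that moves toward a given location.
; DoMove caches the destination and starts a looping timer on UpdateDestLoc, which feeds a normalized, delta-scaled direction into CharacterMovement as input.
; The timer is never cleared here; the Normalize tolerance zeroes the input very near the destination.
; Mesh clicks only print a debug string, and DoMoving is empty.
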(event OnClicked(Mesh)
  (params (TouchedComponent :type Primitive%20Component%20Object%20Reference) (ButtonPressed :type Key%20Structure :default "None"))
  (Development|PrintString "ClickedMesh" true true "(R=1.000000,G=0.000000,B=0.013240,A=1.000000)"))

(fn ConstructionScript)

(fn DoMove
  (params (Location :type Vector))
  (Variables|Default|SetCachedDestLoc Location)
  (Utilities|Time|SetTimerbyFunctionName 0 "UpdateDestLoc" 0.01 true))

(fn UpdateDestLoc
  (Class|PawnMovementComponent|AddInputVector (Variables|Character|GetCharacterMovement) (* (Math|Vector|Normalize (- (Variables|Default|GetCachedDestLoc) (Transformation|GetActorLocation)) 1.0) (* 1e+03 (Utilities|Time|GetWorldDeltaSeconds))) false))

(fn DoMoving)