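; Tile map manager for a turn-based game that generates the tile grid and handles tile selection and path highlighting.
; On BeginPlay it binds itself to the controlled BP_DefaultPawn.
; Selecting a new walkable tile clears the old path, switches the tile visual types and fires a selection dispatcher.
; Paths run from the selected tile to a target in manager-relative coordinates, and their tiles are re-typed to show the route.
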(event EventBeginPlay
  (bind _asbp_default_pawn (Utilities|Casting|CastToBP_DefaultPawn (Pawn|GetControlledPawn (Game|GetPlayerController 0))))
  (Default|BindTileMapManager _asbp_default_pawn self))

(fn ConstructionScript)

(fn CreateTile
  (Class|TileMapManager|GenerateTileMap (Variables|Default|GetMap%20Width) (Variables|Default|GetMap%20Height)))

(fn FindPathtoTile
  (params (TargetTile :type BP%20My%20Tile%20Base%20Object%20Reference))
  (bind _returnvalue (Transformation|GetActorLocation))
  (bind _selectedtile (Variables|Default|GetSelectedTile)
    (:then
      (if (!= _selectedtile TargetTile)
        (CallFunction|ClearPathTile)
        (bind _returnvalue_2 (Class|TileMapManager|FindPath (- (Transformation|GetActorLocation (Variables|Default|GetSelectedTile)) _returnvalue) (- (Transformation|GetActorLocation TargetTile) _returnvalue)))
        (bind _output_get (Variables|Default|SetPathTiles _returnvalue_2))
        (for _array_element _output_get
          (bind _asbp_my_tile_base (Utilities|Casting|CastToBP_MyTileBase _array_element))
          (Default|ChangeTileType _asbp_my_tile_base "NewEnumerator3"))))
    (:else)))

(fn ApplySelectTile
  (params (SelectedTile :type BP%20My%20Tile%20Base%20Object%20Reference))
  (if (and (!= (Variables|Default|GetSelectedTile) SelectedTile) (Variables|/Script/TurnBasedPlugin.TileBase|GetbIsWalkable SelectedTile))
    (Development|PrintString (Utilities|String|Append "SelectedTile - " (Utilities|GetDisplayName SelectedTile)) true true "(R=0.000000,G=0.660000,B=1.000000,A=1.000000)" 2e+01)
    (CallFunction|ClearPathTile)
    (Utilities|FlowControl|Sequence
      (:then_0
        (bind _selectedtile (Variables|Default|GetSelectedTile)
          (:then
            (Default|ChangeTileType _selectedtile "NewEnumerator1"))
          (:else)))
      (:then_1
        (bind _output_get (Variables|Default|SetSelectedTile SelectedTile))
        (Default|ChangeTileType _output_get "NewEnumerator2")
        (Default|CallEventDispatcherSelectTile (Variables|Default|GetSelectedTile))))))

(fn ClearPathTile
  (if (Utilities|Array|IsNotEmpty (Variables|Default|GetPathTiles))
    (Utilities|FlowControl|Sequence
      (:then_0
        (for _array_element (Variables|Default|GetPathTiles)
          (bind _asbp_my_tile_base (Utilities|Casting|CastToBP_MyTileBase _array_element))
          (Default|ChangeTileType _asbp_my_tile_base "NewEnumerator1")))
      (:then_1
        (Utilities|Array|Clear (Variables|Default|GetPathTiles))))))