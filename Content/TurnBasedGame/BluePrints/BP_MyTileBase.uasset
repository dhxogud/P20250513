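; BP_MyTileBase is a tile in the turn-based game's tile map, with walkability, terrain cost and a visual tile type.
; Construction tints its dynamic material by walkability and raises it above the TileMapManager in proportion to terrain cost.
; Cursor hover asks BP_MyTileMapManager to find a path to the tile; clicking does nothing, as the selection logic is disconnected.
; ChangeTileType recolors the tile by state, and GetTileSize derives its width from the box extent.
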(event OnClicked(Cube)
  (params (TouchedComponent :type Primitive%20Component%20Object%20Reference) (ButtonPressed :type Key%20Structure :default "None")))

(event OnBeginCursorOver(Cube)
  (params (TouchedComponent :type Primitive%20Component%20Object%20Reference))
  (bind _asbp_my_tile_map_manager (Utilities|Casting|CastToBP_MyTileMapManager (Variables|Default|GetTileMapManager)))
  (Default|FindPathtoTile _asbp_my_tile_map_manager self))

(event EventBeginPlay
  (bind _cube (Variables|Default|GetCube))
  (bind _returnvalue (Rendering|Material|CreateDynamicMaterialInstance _cube 0 (Rendering|Material|GetMaterial _cube 0) "None" :!class /Script/Engine.PrimitiveComponent))
  (Variables|Default|SetDynamicMaterial _returnvalue))

(fn ConstructionScript
  (bind _returnvalue (Transformation|GetActorLocation))
  (Utilities|FlowControl|Sequence
    (:then_0
      (bind _returnvalue_2 (Rendering|Material|CreateDynamicMaterialInstance (Variables|Default|GetCube) 0 "/TurnBasedPlugin/TurnBasedTemplate/Materials/M_Border_Inst.M_Border_Inst" "None" :!class /Script/Engine.PrimitiveComponent))
      (Variables|Default|SetDynamicMaterial _returnvalue_2))
    (:then_1
      (if (Variables|Default|GetbIsWalkable)
        (Rendering|Material|SetVectorParameterValue (Variables|Default|GetDynamicMaterial) "Color" "(R=1.000000,G=1.000000,B=1.000000,A=1.000000)" :!class /Script/Engine.MaterialInstanceDynamic)
        (else
          (Rendering|Material|SetVectorParameterValue (Variables|Default|GetDynamicMaterial) "Color" "(R=0.000000,G=0.000000,B=0.000000,A=1.000000)" :!class /Script/Engine.MaterialInstanceDynamic))))
    (:then_2
      (bind _tilemapmanager (Variables|Default|GetTileMapManager)
        (:then
          (Transformation|SetActorLocation (Math|Vector|MakeVector (.x _returnvalue) (.y _returnvalue) (+ (.z (Transformation|GetActorLocation _tilemapmanager)) (* (Variables|Default|GetTerrainCost) 20))) false false))
        (:else)))))

(fn ChangeTileType
  (params (TileType :type EN_TileType%20Enum :default "NewEnumerator0"))
  (bind _output_get (Variables|Default|SetTileType TileType))
  (switch Utilities|FlowControl|Switch|SwitchonEN_TileType _output_get
    (:NewEnumerator0
      (Rendering|Material|SetVectorParameterValue :self (Variables|Default|GetDynamicMaterial) :ParameterName "Color" :!class /Script/Engine.MaterialInstanceDynamic))
    (:NewEnumerator1
      (Rendering|Material|SetVectorParameterValue (Variables|Default|GetDynamicMaterial) "Color" "(R=1.000000,G=1.000000,B=1.000000,A=1.000000)" :!class /Script/Engine.MaterialInstanceDynamic))
    (:NewEnumerator2
      (Rendering|Material|SetVectorParameterValue (Variables|Default|GetDynamicMaterial) "Color" "(R=1.000000,G=1.000000,B=0.000000,A=1.000000)" :!class /Script/Engine.MaterialInstanceDynamic))
    (:NewEnumerator3
      (Rendering|Material|SetVectorParameterValue (Variables|Default|GetDynamicMaterial) "Color" "(R=1.000000,G=0.000000,B=0.000000,A=1.000000)" :!class /Script/Engine.MaterialInstanceDynamic))))

(fn GetTileSize
  (return (* (.x (Variables|/Script/Engine.BoxComponent|GetBoxExtent (Variables|Default|GetBox))) 2.0)))