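; Player controller for the turn-based game, turning Enhanced Input into camera and tile-selection commands on the controlled BP_DefaultPawn.
; BeginPlay adds the IMC_TurnBased context; move and zoom input go to the pawn's DoMove and DoZoom.
; Clicks trace under the cursor for a BP_MyTileBase and pass it to the pawn's FindUnitOnTile.
; Destination, touch and cursor-FX helpers exist but no live event calls them.
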(event Input|EnhancedActionEvents|EnhancedInputActionIA_CameraZoom
  (params (ActionValue :type Float%20%28double-precision%29) (ElapsedSeconds :type Float%20%28double-precision%29) (TriggeredSeconds :type Float%20%28double-precision%29) (InputAction :type Input%20Action%20Object%20Reference :default "/Game/TurnBasedGame/Input/Actions/IA_CameraZoom.IA_CameraZoom"))
  ;[0.15 0.15 0.15 0.5] 카메라 Zoom 기능 (Spring Arm Length 조절)
  (bind _asbp_default_pawn (Utilities|Casting|CastToBP_DefaultPawn (Pawn|GetControlledPawn)))
  (Default|DoZoom _asbp_default_pawn ActionValue))

(event Input|EnhancedActionEvents|EnhancedInputActionIA_CameraMove
  (params (ActionValue :type Vector%202D%20Structure) (ElapsedSeconds :type Float%20%28double-precision%29) (TriggeredSeconds :type Float%20%28double-precision%29) (InputAction :type Input%20Action%20Object%20Reference :default "/Game/TurnBasedGame/Input/Actions/IA_CameraMove.IA_CameraMove"))
  ;[0.15 0.15 0.15 0.5] 카메라 WASD 이동 ( XY 평면 수평이동)
  (bind _asbp_default_pawn (Utilities|Casting|CastToBP_DefaultPawn (Pawn|GetControlledPawn)))
  (Default|DoMove _asbp_default_pawn (.x ActionValue) (.y ActionValue)))

(event Input|EnhancedActionEvents|EnhancedInputActionIA_OnClicked
  (params (ActionValue :type Boolean) (ElapsedSeconds :type Float%20%28double-precision%29) (TriggeredSeconds :type Float%20%28double-precision%29) (InputAction :type Input%20Action%20Object%20Reference :default "/Game/TurnBasedGame/Input/Actions/IA_OnClicked.IA_OnClicked"))
  (bind _tile (CallFunction|GetTileUnderCursor))
  ;[0.05098 0.05098 0.05098] OnClicked 이벤트
  (:Started
    (Utilities|IsValid _tile
      (:Is%20Valid
        (bind _asbp_default_pawn (Utilities|Casting|CastToBP_DefaultPawn (Pawn|GetControlledPawn)))
        (Default|FindUnitonTile _asbp_default_pawn _tile)))))

(event Input|EnhancedActionEvents|EnhancedInputActionIA_SetDestination_Click
  (params (ActionValue :type Boolean) (ElapsedSeconds :type Float%20%28double-precision%29) (TriggeredSeconds :type Float%20%28double-precision%29) (InputAction :type Input%20Action%20Object%20Reference :default "/Game/TurnBasedGame/Input/Actions/IA_SetDestination_Click.IA_SetDestination_Click")))

(event EventBeginPlay
  (bind _returnvalue (PlayerController|LocalPlayerSubsystems|GetEnhancedInputLocalPlayerSubsystem))
  ;[0.05098 0.05098 0.05098] Add Mapping Context
  (Utilities|IsValid _returnvalue
    (:Is%20Valid
      (Input|AddMappingContext _returnvalue "/Game/TurnBasedGame/Input/IMC_TurnBased.IMC_TurnBased" 0 "(bIgnoreAllPressedKeysUntilRelease=True,bForceImmediately=False,bNotifyUserSettings=False)"))))

(fn ConstructionScript)

(fn ShowSelectedLocation
  (params (Location :type Vector))
  (Niagara|SpawnSystematLocation (Variables|Input|GetFXCursor) Location))

(fn SelectDestination
  (params (Location :type Vector))
  (bind _asbp_default_pawn (Utilities|Casting|CastToBP_DefaultPawn (Pawn|GetControlledPawn)))
  (Default|PointatLocation _asbp_default_pawn Location))

(fn GetLocationUnderCursor
  (bind _hitresult (Game|Player|GetHitResultUnderCursorbyChannel "TraceTypeQuery1" true))
  (bind (_bblockinghit _binitialoverlap _time _distance _location) (Collision|BreakHitResult _hitresult))
  (return _bblockinghit _location))

(fn GetLocationUnderFinger
  (bind _hitresult (Class|PlayerController|GetHitResultUnderFingerbyChannel "Touch1" "TraceTypeQuery1" false))
  (bind (_bblockinghit _binitialoverlap _time _distance _location) (Collision|BreakHitResult _hitresult))
  (return _bblockinghit _location))

(fn GetTileUnderCursor
  (bind _asbp_my_tile_base (Utilities|Casting|CastToBP_MyTileBase (.HitActor (Collision|BreakHitResult (.HitResult (Game|Player|GetHitResultUnderCursorbyChannel "TraceTypeQuery1" true)))))
    (:then
      (return _asbp_my_tile_base))
    (:CastFailed
      (Development|PrintString "Cast Failed"))))